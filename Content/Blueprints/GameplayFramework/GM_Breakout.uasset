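; Game mode for a Breakout game that sets up the paddle, camera and ball when play begins.
; BeginPlay spawns a paddle at the PS_Player1 player start and has the first player controller possess it.
; It then switches that controller's view to a tagged fixed camera and, after a short delay, spawns a ball at the world origin.
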(event EventBeginPlay
  (Utilities|FlowControl|Sequence
    (:then_0
      (Variables|Default|SetPC0 (Game|GetPlayerController 0)))
    (:then_1
      (bind _returnvalue (Game|SpawnActorfromClass "/Game/Blueprints/BP_BO_Paddle.BP_BO_Paddle_C" (Transformation|GetActorTransform (Class|GameModeBase|FindPlayerStart (Variables|Default|GetPC0) "PS_Player1")) "Undefined" "MultiplyWithRoot" 0 0))
      (Pawn|Possess (Variables|Default|GetPC0) _returnvalue))
    (:then_2
      (bind _outactors (Actor|GetAllActorsOfClasswithTag "/Game/Blueprints/BP_FixedCamera.BP_FixedCamera_C" "FixedCam"))
      (Game|Player|SetViewTargetwithBlend (Variables|Default|GetPC0) (Utilities|Array|Get(acopy) _outactors) 0.0 "VTBlend_Linear" 0.0 false))
    (:then_3
      (Utilities|FlowControl|Delay 1.0)
      (Game|SpawnActorfromClass "/Game/Blueprints/BP_BO_Ball.BP_BO_Ball_C" (Math|Transform|MakeTransform "0, 0, 0") "Undefined" "MultiplyWithRoot" 0 0))))

(fn ConstructionScript)