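; Game mode for Pong that sets up a local two-player match on BeginPlay.
; It creates a second local player, then spawns a paddle at each player's named PlayerStart and possesses it with that player's controller.
; The first controller's view switches to a tagged fixed camera, and a ball spawns at the world origin after a short delay.
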(event EventBeginPlay
  (Utilities|FlowControl|Sequence
    (:then_0
      (Variables|Default|SetPC0 (Game|GetPlayerController 0)))
    (:then_1
      (bind _returnvalue (Class|GameplayStatics|CreatePlayer -1))
      (Variables|Default|SetPC1 _returnvalue))
    (:then_2
      (bind _returnvalue_2 (Game|SpawnActorfromClass "/Game/Blueprints/BP_PongPaddle.BP_PongPaddle_C" (Transformation|GetActorTransform (Class|GameModeBase|FindPlayerStart (Variables|Default|GetPC0) "PS_Player1")) "Undefined" "MultiplyWithRoot" 0 0))
      (Pawn|Possess (Variables|Default|GetPC0) _returnvalue_2))
    (:then_3
      (bind _returnvalue_3 (Game|SpawnActorfromClass "/Game/Blueprints/BP_PongPaddle.BP_PongPaddle_C" (Transformation|GetActorTransform (Class|GameModeBase|FindPlayerStart (Variables|Default|GetPC1) "PS_Player2")) "Undefined" "MultiplyWithRoot" 0 0))
      (Pawn|Possess (Variables|Default|GetPC1) _returnvalue_3))
    (:then_4
      (bind _outactors (Actor|GetAllActorsOfClasswithTag "/Game/Blueprints/BP_FixedCamera.BP_FixedCamera_C" "FixedCam"))
      (Game|Player|SetViewTargetwithBlend (Variables|Default|GetPC0) (Utilities|Array|Get(acopy) _outactors) 0.0 "VTBlend_Linear" 0.0 false))
    (:then_5
      (Utilities|FlowControl|Delay 1.0)
      (Game|SpawnActorfromClass "/Game/Blueprints/BP_PongBall.BP_PongBall_C" (Math|Transform|MakeTransform "0, 0, 0") "Undefined" "MultiplyWithRoot" 0 0))))

(fn ConstructionScript)